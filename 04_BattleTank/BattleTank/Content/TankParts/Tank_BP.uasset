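; Tank Blueprint that sets up the tank's parts and an orbiting, zoomable camera rig.
; On BeginPlay it registers the barrel and turret components through reference setter calls.
; Aim axes yaw an azimuth gimbal and pitch the spring arm separately, scaled by delta time.
; The camera depth axis steps the spring arm length, ignoring changes that would leave a fixed near-to-far range.
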(event `self.ReceiveBeginPlay`
  (`self.SetBarrelReference` (`self.TankBarrel`))
  (`self.SetTurretReference` (`self.TankTurret`)))

(event `InputAxis|AimAzimuth`
  (params (AxisValue :type "Float (single-precision)"))
  ;[1 1 1] Camera Input Binding
  (`SceneComponent.K2_AddLocalRotation` (`self.Azimuth Gibmal`) (`KismetMathLibrary.MakeRotator` 0.0 0.0 (* AxisValue (`GameplayStatics.GetWorldDeltaSeconds`) 100.0)) false false))

(event `InputAxis|AimElevation`
  (params (AxisValue :type "Float (single-precision)"))
  ;[1 1 1] Camera Input Binding
  (`SceneComponent.K2_AddLocalRotation` (`self.SpringArm`) (`KismetMathLibrary.MakeRotator` 0.0 (* AxisValue (`GameplayStatics.GetWorldDeltaSeconds`) 100.0)) false false))

(event `InputAxis|CameraDepth`
  (params (AxisValue :type "Float (single-precision)"))
  (bind _output_get (set `self.SpringSize` (+ (* AxisValue -100.0) (`SpringArmComponent.TargetArmLength` (`self.SpringArm`)) 0.0)))
  (if (<= _output_get 2500.0)
    (if (>= _output_get 600.0)
      (set `SpringArmComponent.TargetArmLength` _output_get (`self.SpringArm`)))))

(fn `UserConstructionScript`)